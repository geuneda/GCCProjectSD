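; BP_WeaponAR is a hitscan weapon Blueprint that deals damage along a line trace when it attacks.
; Its Attack override calls the parent with a zero vector, then traces on the Visibility channel from the Arrow component to the Target location, with one-frame debug drawing.
; It applies fixed damage to the hit actor, naming itself as damage causer, without branching on the trace result.
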(fn `Attack`
  (params (Target :type "Vector Structure"))
  (`parent.Attack` (0.0 0.0 0.0))
  (bind _outhit (`KismetSystemLibrary.LineTraceSingle` :`Start` (`SceneComponent.K2_GetComponentLocation` (`self.Arrow`)) :`End` Target :`TraceChannel` "TraceTypeQuery1" :`DrawDebugType` "ForOneFrame"))
  (`GameplayStatics.ApplyDamage` (`.HitActor` (`GameplayStatics.BreakHitResult` _outhit)) 10.0 null self))

(fn `UserConstructionScript`
  (`parent.UserConstructionScript`))