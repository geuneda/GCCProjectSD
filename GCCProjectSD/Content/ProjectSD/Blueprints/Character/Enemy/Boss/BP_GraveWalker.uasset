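; Grave Walker boss enemy with destructible weak-point parts, a main health pool and a camera-facing health bar.
; BeginPlay builds the weak-point array and triggers slug and javelin shots.
; Point damage always reduces main health; hit parts either flash through a timeline-driven Material Parameter Collection color or detach with physics and are destroyed after a delay.
; Death currently only prints a message.
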(event `self.ReceiveBeginPlay`
  (`|ExecutionSequence`
    (:`then_0`
      ; 파괴 가능 부위 구조체 초기화
      (set `self.weakPoints` (`|MakeArray` (make `/Game/ProjectSD/Blueprints/Structure/FWeakPointData` (`self.BOS_1001_A001_Right_Crab_parts`) 500.0 500.0) (make `/Game/ProjectSD/Blueprints/Structure/FWeakPointData` (`self.BOS_1001_A001_Right_Crab_parts`) 500.0 500.0) (make `/Game/ProjectSD/Blueprints/Structure/FWeakPointData` (`self.BOS_1001_A001_FrontCore01_Parts`) 500.0 500.0) (make `/Game/ProjectSD/Blueprints/Structure/FWeakPointData` (`self.BOS_1001_A001_Right_KneeItem01_parts`) 500.0 500.0) (make `/Game/ProjectSD/Blueprints/Structure/FWeakPointData` (`self.BOS_1001_A001_Right_KneeItem02_parts`) 500.0 500.0) (make `/Game/ProjectSD/Blueprints/Structure/FWeakPointData` (`self.BOS_1001_A001_Right_KneeItem03_parts`) 500.0 500.0) (make `/Game/ProjectSD/Blueprints/Structure/FWeakPointData` (`self.BOS_1001_A001_Left_KneeItem04_parts`) 500.0 500.0) (make `/Game/ProjectSD/Blueprints/Structure/FWeakPointData` (`self.BOS_1001_A001_Left_KneeItem05_parts`) 500.0 500.0) (make `/Game/ProjectSD/Blueprints/Structure/FWeakPointData` (`self.BOS_1001_A001_Left_KneeItem06_parts`) 500.0 500.0))))
    (:`then_1`
      (`KismetSystemLibrary.Delay` 0.5)
      (`self.LSlugShot`)
      (`KismetSystemLibrary.Delay` 0.5)
      (`self.RSlugShot`)
      (`self.LJavelinShotStart`))))

(event `self.ReceiveTick`
  (params (DeltaSeconds :type "Float (single-precision)"))
  (bind _hpbar (`self.HpBar`))
  (`|ExecutionSequence`
    (:`then_0`
      ; UI회전 (체력바, 이름 등)
      (bind _aswbp_boss_hp (cast `/Game/ProjectSD/Blueprints/UI/Enemy/BossEnemy/WBP_BossHP` (`WidgetComponent.GetWidget` _hpbar)))
      (`ProgressBar.SetPercent` (`/Game/ProjectSD/Blueprints/UI/Enemy/BossEnemy/WBP_BossHP.BossHealthBar` _aswbp_boss_hp) (/ (`self.CurrentHealth`) (`self.MaxHealth`)))
      (`SceneComponent.K2_SetWorldRotation` _hpbar (`KismetMathLibrary.FindLookAtRotation` (`SceneComponent.K2_GetComponentLocation` _hpbar) (`SceneComponent.K2_GetComponentLocation` (`PlayerCameraManager.TransformComponent` (`GameplayStatics.GetPlayerCameraManager` 0)))) false false))))

(event `self.ReceivePointDamage`
  (params (Damage :type "Float (single-precision)") (DamageType :type "DamageType Object Reference") (HitLocation :type "Vector Structure") (HitNormal :type "Vector Structure") (HitComponent :type "PrimitiveComponent Object Reference") (BoneName :type Name) (ShotFromDirection :type "Vector Structure") (InstigatedBy :type "Controller Object Reference") (DamageCauser :type "Actor Object Reference") (HitInfo :type "HitResult Structure (by ref)"))
  (bind _weakpoints (`self.weakPoints`))
  ; 부위별 데미지
  (for (_array_element _array_index) _weakpoints
    (bind (_meshcomp _currenthealth _maxhealth) (break `/Game/ProjectSD/Blueprints/Structure/FWeakPointData` _array_element))
    (if (== _meshcomp HitComponent)
      (bind _returnvalue (- _currenthealth Damage))
      ;; 파괴 or 데미지 분기점
      (if (<= _returnvalue 0.0)
        ; 부위 파괴시키는 함수
        (bind _part (`self.DestroyPart` _meshcomp))
        (`KismetSystemLibrary.Delay` 3.0)
        (`ActorComponent.K2_DestroyComponent` _part)
        (else
          (`KismetArrayLibrary.Array_Set` _weakpoints _array_index (make `/Game/ProjectSD/Blueprints/Structure/FWeakPointData` _meshcomp _returnvalue _maxhealth))
          (`self.ApplyPartDamage` _meshcomp)))))
  ; 본체 데미지 (항상)
  (`self.TakeDamage` Damage))

(event `ApplyPartDamage`
  (params (PartSkeltal :type "SkeletalMeshComponent Object Reference"))
  ; 피격 부위 색상 적용
  (bind (_direction _changedtime) (`Timeline|Timeline_0` :!via `PlayFromStart`)
    (:`Update`
      (`self.ChangeMaterial` PartSkeltal PartSkeltal _changedtime))))

(fn `ChangeMaterial`
  (params (Primitive :type "PrimitiveComponent Object Reference") (Mesh :type "MeshComponent Object Reference") (Color :type "Float (double-precision)"))
  (`/Engine/EditorBlueprintResources/StandardMacros.IsValid` Primitive
    (:`Is Valid`
      (`/Engine/EditorBlueprintResources/StandardMacros.IsValid` Mesh
        (:`Is Valid`
          (`self.SetMaterialParamName` Mesh Mesh)
          (`KismetMaterialLibrary.SetVectorParameterValue` "/Game/ProjectSD/Blueprints/MPC_BossColor.MPC_BossColor" (`self.Parameter Name`) (make `LinearColor` Color Color 0.0 1.0)))))))

(fn `DestroyPart`
  (params (PartMesh :type "SkeletalMeshComponent Object Reference"))
  (returns (Part :type "SkeletalMeshComponent Object Reference"))
  (`SceneComponent.K2_DetachFromComponent` PartMesh "KeepRelative" "KeepRelative" "KeepRelative" true)
  (`PrimitiveComponent.SetSimulatePhysics` PartMesh true)
  (return PartMesh))

(fn `Die`
  (`KismetSystemLibrary.PrintString` "죽음"))

(fn `SetMaterialParamName`
  (params (A :type "Object Object Reference") (A2 :type "Object Object Reference"))
  (if (== A2 (`self.BOS_1001_A001_FrontCore01_Parts`))
    (set `self.Parameter Name` "CenterColor")
    (elif (== A (`self.BOS_1001_A001_Left_Crab_parts`))
      (set `self.Parameter Name` "LeftColor")
      (else
        (set `self.Parameter Name` "RightColor")))))

(fn `TakeDamage`
  (params (Damage :type "Float (double-precision)"))
  (bind _output_get (set `self.CurrentHealth` (- (`self.CurrentHealth`) Damage)))
  (if (<= _output_get 0.0)
    (`self.Die`)))

(fn `UserConstructionScript`)