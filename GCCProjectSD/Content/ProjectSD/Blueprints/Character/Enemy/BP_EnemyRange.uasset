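; BP_EnemyRange is a ranged enemy that shoots the player with a hitscan attack, built on parent Spawn and Die logic.
; Attack plays a montage and fires a Visibility line trace from the muzzle socket toward the player, damaging on hit.
; It signals attack end when the montage completes or is interrupted.
; Death triggers a timeline-driven material dissolve through the MeleeDissolve parameter collection, with a short lifespan before removal.
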(event `Dissolve_Event`
  ; 디졸브 효과
  (for _index (range (+ (`PrimitiveComponent.GetNumMaterials` (`self.Mesh`)) 1))
    (`PrimitiveComponent.SetMaterial` (`self.Mesh`) _index "/Game/ProjectSD/Resources/Dissolve/M_DissolveMelee.M_DissolveMelee")
    (bind (_direction _dissolvevalue) (`Timeline|Timeline` :!via `PlayFromStart`)
      (:`Update`
        (`KismetMaterialLibrary.SetScalarParameterValue` "/Game/ProjectSD/Resources/Dissolve/MeleeDissolve.MeleeDissolve" "Value" _dissolvevalue)
        (`self.SetLifeSpan` 2.0)))))

(event `Attack`
  (bind _mesh (`self.Mesh`))
  (`|PlayMontage` (`self.Mesh`) "/Game/ProjectSD/Resources/Characters/Monster/Ranged/Montage/AttackMontage.AttackMontage"
    (:`then`
      (`self.Fire` 10.0 (`SkeletalMeshSocket.GetSocketLocation` (`SkinnedAsset.FindSocket` (`SkinnedMeshComponent.SkinnedAsset` _mesh) "MuzzleSocket") _mesh) (`self.K2_GetActorLocation` (`GameplayStatics.GetPlayerCharacter` 0))))
    (:`OnCompleted`
      (`self.OnAttackEnd` :!label _label))
    (:`OnInterrupted`
      (goto _label))))

(event `self.ReceiveBeginPlay`
  (`self.Spawn` (`self.RangedAttackRange`)))

(fn `Die`
  (`self.Dissolve_Event`)
  (`parent.Die`))

(fn `Fire`
  (params (Damage :type "Float (double-precision)") (StartPoint :type "Vector Structure") (TargetPoint :type "Vector Structure"))
  (bind _outhit (`KismetSystemLibrary.LineTraceSingle` :`Start` StartPoint :`End` TargetPoint :`TraceChannel` "TraceTypeQuery1" :`DrawDebugType` "ForOneFrame"))
  (bind _asbp_player_character (cast `/Game/ProjectSD/Blueprints/Character/Player/BP_PlayerCharacter` (`.HitActor` (`GameplayStatics.BreakHitResult` _outhit))))
  (`GameplayStatics.ApplyDamage` _asbp_player_character Damage))

(fn `Spawn`
  (params (AttackRange :type "Float (double-precision)"))
  (`parent.Spawn` AttackRange))

(fn `UserConstructionScript`
  (`parent.UserConstructionScript`))