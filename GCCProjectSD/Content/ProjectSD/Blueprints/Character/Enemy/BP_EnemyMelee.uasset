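; Melee enemy Blueprint that spawns with a melee attack range and default controller, attacks, and dissolves on death.
; Attack plays a montage unless the game mode reports the game is set, then signals attack end on completion or interruption.
; Die triggers a timeline-driven dissolve that swaps every mesh material to the ranged dissolve material, animates a shared parameter collection and sets a short lifespan.
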(event `Dissolve_Event`
  ; 디졸브 효과
  (for _index (range (+ (`PrimitiveComponent.GetNumMaterials` (`self.Mesh`)) 1))
    (`PrimitiveComponent.SetMaterial` (`self.Mesh`) _index "/Game/ProjectSD/Resources/Dissolve/M_DissolveRanged.M_DissolveRanged")
    (bind (_direction _dissolvevalue) (`Timeline|Timeline` :!via `PlayFromStart`)
      (:`Update`
        (`KismetMaterialLibrary.SetScalarParameterValue` "/Game/ProjectSD/Resources/Dissolve/RangedDissolve.RangedDissolve" "Value" _dissolvevalue)
        (`self.SetLifeSpan` 2.0)))))

(event `Attack`
  (bind _asbp_sdgame_mode (cast `/Game/ProjectSD/Blueprints/BP_SDGameMode` (`GameplayStatics.GetGameMode`)))
  (if (not (`/Game/ProjectSD/Blueprints/BP_SDGameMode.bIsGameSet` _asbp_sdgame_mode))
    (`|PlayMontage` (`self.Mesh`) "/Game/ProjectSD/Resources/Characters/Monster/Melee/Montage/AttackMontage.AttackMontage"
      (:`OnCompleted`
        _)
      (:`OnInterrupted`
        _))
    (`self.OnAttackEnd`)))

(event `self.ReceiveBeginPlay`
  (`|ExecutionSequence`
    (:`then_0`
      (`self.Spawn` (`self.MeleeAttackRange`)))
    (:`then_1`
      (`self.SpawnDefaultController`))))

(fn `Die`
  (`self.Dissolve_Event`)
  (`parent.Die`))

(fn `Spawn`
  (params (AttackRange :type "Float (double-precision)"))
  (`parent.Spawn` AttackRange))

(fn `UserConstructionScript`
  (`parent.UserConstructionScript`))