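; Base enemy character with a stats struct, an overhead health bar, damage handling and a player-chase behavior.
; BeginPlay fills the stats through Spawn and caches the player, while Tick refreshes the health bar and turns it toward the camera.
; AnyDamage subtracts health, or triggers a ragdoll death with capsule collision disabled when damage exceeds it.
; ChasePlayer, not called here, repeats AI MoveTo after a delay on each success.
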(event `self.ReceiveBeginPlay`
  (`self.Spawn` 0.0)
  (set `self.Player` (`GameplayStatics.GetPlayerCharacter` 0)))

(event `self.ReceiveTick`
  (params (DeltaSeconds :type "Float (single-precision)"))
  (bind _healthwidget (`self.Healthwidget`))
  (`|ExecutionSequence`
    (:`then_0`
      ; UI회전 (체력바, 이름 등)
      (`self.SetHpBar`)
      (`SceneComponent.K2_SetWorldRotation` _healthwidget (`KismetMathLibrary.FindLookAtRotation` (`SceneComponent.K2_GetComponentLocation` _healthwidget) (`SceneComponent.K2_GetComponentLocation` (`PlayerCameraManager.TransformComponent` (`GameplayStatics.GetPlayerCameraManager` 0)))) false false))))

(event `self.ReceiveAnyDamage`
  (params (Damage :type "Float (single-precision)") (DamageType :type "DamageType Object Reference") (InstigatedBy :type "Controller Object Reference") (DamageCauser :type "Actor Object Reference"))
  (bind (_currenthealth _maxhealth _attackpower _movespeed _isdead _attackranged) (break `/Game/ProjectSD/Blueprints/Structure/EnemyBaseStat` (`self.EnemyStat`)))
  (bind _returnvalue (- _currenthealth Damage))
  ; TakeDamage 구현
  (if (>= _returnvalue 0.0)
    (set `self.EnemyStat` (make `/Game/ProjectSD/Blueprints/Structure/EnemyBaseStat` _returnvalue _maxhealth _attackpower _movespeed _isdead _attackranged))
    (else
      (`self.SetHpBar`)
      (`self.Die`))))

(event `ChasePlayer`
  (`|AIMoveTo` self (0.0 0.0 0.0) (`self.Player`) 150.0
    (:`OnSuccess`
      (`KismetSystemLibrary.Delay` 2.0)
      (`self.ChasePlayer`))))

(fn `Die`
  (bind _mesh (`self.Mesh`))
  (`PrimitiveComponent.SetSimulatePhysics` _mesh true)
  (`PrimitiveComponent.SetCollisionEnabled` (`self.CapsuleComponent`) "NoCollision")
  (`PrimitiveComponent.SetCollisionEnabled` _mesh "QueryAndPhysics"))

(fn `SetHpBar`
  (bind (_enemystat_currenthealth _enemystat_maxhealth) (break `/Game/ProjectSD/Blueprints/Structure/EnemyBaseStat` (`self.EnemyStat`)))
  (bind _aswbp_enemy_hpbar (cast `/Game/ProjectSD/Blueprints/UI/Enemy/NormalEnemy/WBP_EnemyHPBar` (`WidgetComponent.GetWidget` (`self.Healthwidget`))))
  (`ProgressBar.SetPercent` (`/Game/ProjectSD/Blueprints/UI/Enemy/NormalEnemy/WBP_EnemyHPBar.HealthBar` _aswbp_enemy_hpbar) (/ _enemystat_currenthealth _enemystat_maxhealth)))

(fn `Spawn`
  (params (AttackRange :type "Float (double-precision)"))
  (set `self.EnemyStat` (make `/Game/ProjectSD/Blueprints/Structure/EnemyBaseStat` 500.0 500.0 10.0 100.0 false AttackRange)))

(fn `UserConstructionScript`)