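; Bunny's player skill set, built around an electric force gauge that charges with distance moved and drains while idle.
; C toggles a mentality-draining speed boost that adds charge.
; Z spends charge on a slowing, timer-driven hand beam, aimed by camera trace, damaging via sphere trace at time-ranked strength.
; Completed-jump landings trigger a capsule-overlap shockwave on nearest enemies; Tick updates cooldowns, passive and HUD, while Q and V are stubs.
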(event `self.ReceiveBeginPlay`
  (bind _targetcharacter (`self.TargetCharacter`))
  ; 땅 착지 기능 델리게이트 등록
  (`parent.ReceiveBeginPlay`)
  (add `/Game/ProjectSD/Blueprints/Character/Player/BP_PlayerCharacter.DoOnLanded` (`self.TargetCharacter`) (`|CreateDelegate` :!event `DoOnLandedInterface`))
  ; 패시브 UI
  (bind _returnvalue (`|CreateWidget` "/Game/ProjectSD/Blueprints/Character/Player/PlayerSkill/PlayerSkillUI/BP_BunnySkillPassive.BP_BunnySkillPassive_C"))
  (bind _output_get (set `self.ElectricForceWidget` _returnvalue))
  (`UserWidget.AddToViewport` _output_get 0)
  (bind _returnvalue_2 (`|SpawnActorFromClass` "/Game/ProjectSD/Blueprints/Character/Player/PlayerSkill/EachSkillActor/BP_ZSkillBeamActor.BP_ZSkillBeamActor_C" (`KismetMathLibrary.MakeTransform` (`SceneComponent.GetSocketLocation` (`Character.Mesh` _targetcharacter) "Hook")) "Undefined" "MultiplyWithRoot" _targetcharacter null))
  (set `self.ZSkillBeamActor` _returnvalue_2)
  (`Actor.K2_AttachToActor` _returnvalue_2 _targetcharacter "None" "KeepWorld" "KeepWorld" "KeepWorld" true)
  (bind _returnvalue_3 (`|CreateWidget` "/Game/ProjectSD/Blueprints/Character/Player/PlayerSkill/PlayerSkillUI/WB_BunnySkill.WB_BunnySkill_C"))
  (bind _output_get_2 (set `self.SkillWidget` _returnvalue_3))
  (`UserWidget.AddToViewport` _output_get_2 0)
  (bind _returnvalue_4 (`GameplayStatics.SpawnSound2D` "/Game/Resources/Sounds/Player/Skill4/PC_Se_Bunny_Active4_Beam_LP.PC_Se_Bunny_Active4_Beam_LP" 1.0 1.0 0.0 null false false))
  (bind _output_get_3 (set `self.BeamSound` _returnvalue_4))
  (`AudioComponent.Stop` _output_get_3))

(event `self.ReceiveTick`
  (params (DeltaSeconds :type "Float (single-precision)"))
  (`parent.ReceiveTick` DeltaSeconds)
  (`|ExecutionSequence`
    (:`then_0`
      (`self.CheckCSkillCoolTime` DeltaSeconds))
    (:`then_1`
      (`self.CheckZSkillCoolTime` DeltaSeconds))
    (:`then_2`
      (`self.PassiveTick` DeltaSeconds)
      (`|ExecutionSequence`
        (:`then_0`
          (`self.CheckSetCSkillCostUI`))
        (:`then_1`
          (`self.CheckSetZSkillCostUI`))))))

(event `QSkillTick`
  (params (NewParam :type "Float (double-precision)")))

(event `Key|Enter`
  (params (Key :type "Key Structure"))
  (:`Pressed`
    (`/Game/ProjectSD/Blueprints/Character/Player/BP_PlayerCharacter.AddMentality` (`self.TargetCharacter`) 50.0)))

(fn `ActionCSkill`
  (bind (_zskillinfo_isaction _zskillinfo_isactioncooltime _zskillinfo_currentcooltime _zskillinfo_maxcooltime _zskillinfo_electricforceconsumptionpersecond _zskillinfo_onoff) (break `/Game/ProjectSD/Blueprints/Character/Player/PlayerSkill/EachSkillStructure/BunnyZSkillInfoBase` (`self.ZSkillInfo`)))
  (bind (_cskillinfo_isaction _cskillinfo_isactioncooltime _cskillinfo_currentcooltime _cskillinfo_maxcooltime _cskillinfo_mentalityconsumption _cskillinfo_onoff _cskillinfo_mentalityconsumptionperseconds _cskillinfo_speedupratio _cskillinfo_gainelectricforceratio) (break `/Game/ProjectSD/Blueprints/Character/Player/PlayerSkill/EachSkillStructure/BunnyCSkillInfo` (`self.CSkillInfo`)))
  (bind (_cskillinfo_isaction_2 _cskillinfo_isactioncooltime_2 _cskillinfo_currentcooltime_2 _cskillinfo_maxcooltime_2 _cskillinfo_mentalityconsumption_2 _cskillinfo_onoff_2) (break `/Game/ProjectSD/Blueprints/Character/Player/PlayerSkill/EachSkillStructure/BunnyCSkillInfo` (`self.CSkillInfo`)))
  (`parent.ActionCSkill`)
  (if _zskillinfo_onoff
    (`KismetSystemLibrary.PrintString` "ZSkill Use!!")
    (elif _cskillinfo_onoff_2
      (`self.CSkillOff`)
      (elif _cskillinfo_isactioncooltime_2
        (bind _isremovable (`/Game/ProjectSD/Blueprints/Character/Player/BP_PlayerCharacter.RemoveMentality` (`self.TargetCharacter`) _cskillinfo_mentalityconsumption_2))
        (if _isremovable
          (`self.CSkillOn`)
          (`KismetSystemLibrary.PrintString` "2번스킬 : 발동!")
          (else
            (set `self.CSkillInfo` (make `/Game/ProjectSD/Blueprints/Character/Player/PlayerSkill/EachSkillStructure/BunnyCSkillInfo` false _cskillinfo_isactioncooltime _cskillinfo_currentcooltime _cskillinfo_maxcooltime _cskillinfo_mentalityconsumption _cskillinfo_onoff _cskillinfo_mentalityconsumptionperseconds _cskillinfo_speedupratio _cskillinfo_gainelectricforceratio))
            (`KismetSystemLibrary.PrintString` "2번스킬 : 정신력 부족!")))
        (else
          (`KismetSystemLibrary.PrintString` "2번스킬 : 쿨타임 대기!!"))))))

(fn `ActionQSkill`
  (bind (_zskillinfo_isaction _zskillinfo_isactioncooltime _zskillinfo_currentcooltime _zskillinfo_maxcooltime _zskillinfo_electricforceconsumptionpersecond _zskillinfo_onoff) (break `/Game/ProjectSD/Blueprints/Character/Player/PlayerSkill/EachSkillStructure/BunnyZSkillInfoBase` (`self.ZSkillInfo`)))
  (`parent.ActionQSkill`)
  (if _zskillinfo_onoff
    _))

(fn `ActionVSkill`
  (`parent.ActionVSkill`))

(fn `ActionZSkill`
  (bind (_zskillinfo_isaction _zskillinfo_isactioncooltime _zskillinfo_currentcooltime _zskillinfo_maxcooltime _zskillinfo_electricforceconsumptionpersecond _zskillinfo_onoff) (break `/Game/ProjectSD/Blueprints/Character/Player/PlayerSkill/EachSkillStructure/BunnyZSkillInfoBase` (`self.ZSkillInfo`)))
  (bind (_zskillinfo_isaction_2 _zskillinfo_isactioncooltime_2 _zskillinfo_currentcooltime_2 _zskillinfo_maxcooltime_2 _zskillinfo_electricforceconsumptionpersecond_2 _zskillinfo_onoff_2 _zskillinfo_speeddownratio _zskillinfo_currentticktime _zskillinfo_attackrank) (break `/Game/ProjectSD/Blueprints/Character/Player/PlayerSkill/EachSkillStructure/BunnyZSkillInfoBase` (`self.ZSkillInfo`)))
  (`parent.ActionZSkill`)
  (if _zskillinfo_onoff
    (`self.ZSkillOff`)
    (elif _zskillinfo_isactioncooltime
      (if (>= (`self.CurrentElectricForce`) _zskillinfo_electricforceconsumptionpersecond)
        (`self.ZSkillOn`)
        (`KismetSystemLibrary.PrintString` "4번스킬 : 발동!")
        (else
          (set `self.ZSkillInfo` (make `/Game/ProjectSD/Blueprints/Character/Player/PlayerSkill/EachSkillStructure/BunnyZSkillInfoBase` false _zskillinfo_isactioncooltime_2 _zskillinfo_currentcooltime_2 _zskillinfo_maxcooltime_2 _zskillinfo_electricforceconsumptionpersecond_2 _zskillinfo_onoff_2 _zskillinfo_speeddownratio _zskillinfo_currentticktime _zskillinfo_attackrank))
          (`KismetSystemLibrary.PrintString` "4번스킬 : 전기력 부족!")))
      (else
        (`KismetSystemLibrary.PrintString` "4번스킬 : 쿨타임 대기!!")))))

(fn `CheckCSkillCoolTime`
  (params (DeltaTime :type "Float (double-precision)"))
  (bind (_cskillinfo_isaction _cskillinfo_isactioncooltime _cskillinfo_currentcooltime _cskillinfo_maxcooltime _cskillinfo_mentalityconsumption _cskillinfo_onoff _cskillinfo_mentalityconsumptionperseconds _cskillinfo_speedupratio _cskillinfo_gainelectricforceratio) (break `/Game/ProjectSD/Blueprints/Character/Player/PlayerSkill/EachSkillStructure/BunnyCSkillInfo` (`self.CSkillInfo`)))
  (bind (_isaction _isactioncooltime _currentcooltime _maxcooltime) (break `/Game/ProjectSD/Blueprints/Character/Player/PlayerSkill/EachSkillStructure/BunnyCSkillInfo` (`self.CSkillInfo`)))
  (bind (_iscompleted _nextcooltime) (`self.CalculateCoolTime` DeltaTime _cskillinfo_currentcooltime _cskillinfo_maxcooltime))
  (set `self.CSkillInfo` (make `/Game/ProjectSD/Blueprints/Character/Player/PlayerSkill/EachSkillStructure/BunnyCSkillInfo` _cskillinfo_isaction _iscompleted _nextcooltime _cskillinfo_maxcooltime _cskillinfo_mentalityconsumption _cskillinfo_onoff _cskillinfo_mentalityconsumptionperseconds _cskillinfo_speedupratio _cskillinfo_gainelectricforceratio))
  (`/Game/ProjectSD/Blueprints/Character/Player/PlayerSkill/PlayerSkillUI/WB_BunnySkill.SetCSkillCoolTimeRatio` (`self.SkillWidget`) _currentcooltime _maxcooltime))

(fn `CheckSetCSkillCostUI`
  (bind _skillwidget (`self.SkillWidget`))
  (bind (_isaction _isactioncooltime _currentcooltime _maxcooltime _mentalityconsumption _onoff) (break `/Game/ProjectSD/Blueprints/Character/Player/PlayerSkill/EachSkillStructure/BunnyCSkillInfo` (`self.CSkillInfo`)))
  (if (and (> _mentalityconsumption (`/Game/ProjectSD/Blueprints/Character/Player/BP_PlayerCharacter.CurrentMentality` (`self.TargetCharacter`))) (not _onoff))
    (`/Game/ProjectSD/Blueprints/Character/Player/PlayerSkill/PlayerSkillUI/WB_BunnySkill.SetCSkillCostOut` _skillwidget true)
    (else
      (`/Game/ProjectSD/Blueprints/Character/Player/PlayerSkill/PlayerSkillUI/WB_BunnySkill.SetCSkillCostOut` _skillwidget false))))

(fn `CheckSetZSkillCostUI`
  (bind _skillwidget (`self.SkillWidget`))
  (bind (_isaction _isactioncooltime _currentcooltime _maxcooltime _electricforceconsumptionpersecond _onoff) (break `/Game/ProjectSD/Blueprints/Character/Player/PlayerSkill/EachSkillStructure/BunnyZSkillInfoBase` (`self.ZSkillInfo`)))
  (if (and (> _electricforceconsumptionpersecond (`self.CurrentElectricForce`)) (not _onoff))
    (`/Game/ProjectSD/Blueprints/Character/Player/PlayerSkill/PlayerSkillUI/WB_BunnySkill.SetZSkillCostOut` _skillwidget true)
    (else
      (`/Game/ProjectSD/Blueprints/Character/Player/PlayerSkill/PlayerSkillUI/WB_BunnySkill.SetZSkillCostOut` _skillwidget false))))

(fn `CheckZSkillCoolTime`
  (params (DeltaTime :type "Float (double-precision)"))
  (bind (_zskillinfo_isaction _zskillinfo_isactioncooltime _zskillinfo_currentcooltime _zskillinfo_maxcooltime _zskillinfo_electricforceconsumptionpersecond _zskillinfo_onoff _zskillinfo_speeddownratio _zskillinfo_currentticktime) (break `/Game/ProjectSD/Blueprints/Character/Player/PlayerSkill/EachSkillStructure/BunnyZSkillInfoBase` (`self.ZSkillInfo`)))
  (bind (_isaction _isactioncooltime _currentcooltime _maxcooltime) (break `/Game/ProjectSD/Blueprints/Character/Player/PlayerSkill/EachSkillStructure/BunnyZSkillInfoBase` (`self.ZSkillInfo`)))
  (bind (_iscompleted _nextcooltime) (`self.CalculateCoolTime` DeltaTime _zskillinfo_currentcooltime _zskillinfo_maxcooltime))
  (set `self.ZSkillInfo` (make `/Game/ProjectSD/Blueprints/Character/Player/PlayerSkill/EachSkillStructure/BunnyZSkillInfoBase` _zskillinfo_isaction _iscompleted _nextcooltime _zskillinfo_maxcooltime _zskillinfo_electricforceconsumptionpersecond _zskillinfo_onoff _zskillinfo_speeddownratio _zskillinfo_currentticktime))
  (`/Game/ProjectSD/Blueprints/Character/Player/PlayerSkill/PlayerSkillUI/WB_BunnySkill.SetZSkillCoolTimeRatio` (`self.SkillWidget`) _currentcooltime _maxcooltime))

(fn `ConsumeElectricForcePerSecond`
  (params (ConsumptionPerSecond :type "Float (double-precision)") (DeltaTime :type "Float (double-precision)"))
  (returns (IsCompleted :type Boolean))
  (locals (TemptConsumption :type "Float (double-precision)"))
  (bind _currentelectricforce (`self.CurrentElectricForce`))
  (bind _temptconsumption (`local.TemptConsumption`))
  (set `local.TemptConsumption` (* (`local.ConsumptionPerSecond`) (`local.DeltaTime`)))
  (if (>= _currentelectricforce _temptconsumption)
    (set `self.CurrentElectricForce` (`KismetMathLibrary.FClamp` (- _currentelectricforce _temptconsumption) 0.0 (`self.MaxElectricForce`)))
    (return true)
    (else
      (return false))))

(fn `CSkillOff`
  (bind _targetcharacter (`self.TargetCharacter`))
  (bind (_cskillinfo_isaction _cskillinfo_isactioncooltime _cskillinfo_currentcooltime _cskillinfo_maxcooltime _cskillinfo_mentalityconsumption _cskillinfo_onoff) (break `/Game/ProjectSD/Blueprints/Character/Player/PlayerSkill/EachSkillStructure/BunnyCSkillInfo` (`self.CSkillInfo`)))
  (bind (_cskillinfo_isaction_2 _cskillinfo_isactioncooltime_2 _cskillinfo_currentcooltime_2 _cskillinfo_maxcooltime_2 _cskillinfo_mentalityconsumption_2 _cskillinfo_onoff_2 _cskillinfo_mentalityconsumptionperseconds _cskillinfo_speedupratio _cskillinfo_gainelectricforceratio) (break `/Game/ProjectSD/Blueprints/Character/Player/PlayerSkill/EachSkillStructure/BunnyCSkillInfo` (`self.CSkillInfo`)))
  (if _cskillinfo_onoff
    (set `CharacterMovementComponent.MaxWalkSpeed` (`/Game/ProjectSD/Blueprints/Character/Player/BP_PlayerCharacter.DefaultMaxSpeed` _targetcharacter) (`Character.CharacterMovement` _targetcharacter))
    (`KismetSystemLibrary.K2_ClearAndInvalidateTimerHandle` (`self.CSkillTickHandler`))
    (set `self.CSkillInfo` (make `/Game/ProjectSD/Blueprints/Character/Player/PlayerSkill/EachSkillStructure/BunnyCSkillInfo` _cskillinfo_isaction_2 false 0.0 _cskillinfo_maxcooltime_2 _cskillinfo_mentalityconsumption_2 false _cskillinfo_mentalityconsumptionperseconds _cskillinfo_speedupratio _cskillinfo_gainelectricforceratio))))

(fn `CSkillOn`
  (locals (CSkillTickFunctionName :type String :default "CSkillTick"))
  (bind (_cskillinfo_isaction _cskillinfo_isactioncooltime _cskillinfo_currentcooltime _cskillinfo_maxcooltime _cskillinfo_mentalityconsumption _cskillinfo_onoff _cskillinfo_mentalityconsumptionperseconds _cskillinfo_speedupratio _cskillinfo_gainelectricforceratio) (break `/Game/ProjectSD/Blueprints/Character/Player/PlayerSkill/EachSkillStructure/BunnyCSkillInfo` (`self.CSkillInfo`)))
  (bind (_cskillinfo_isaction_2 _cskillinfo_isactioncooltime_2 _cskillinfo_currentcooltime_2 _cskillinfo_maxcooltime_2 _cskillinfo_mentalityconsumption_2 _cskillinfo_onoff_2 _cskillinfo_mentalityconsumptionperseconds_2 _cskillinfo_speedupratio_2) (break `/Game/ProjectSD/Blueprints/Character/Player/PlayerSkill/EachSkillStructure/BunnyCSkillInfo` (`self.CSkillInfo`)))
  (bind _charactermovement (`Character.CharacterMovement` (`self.TargetCharacter`)))
  (set `CharacterMovementComponent.MaxWalkSpeed` (* (`CharacterMovementComponent.MaxWalkSpeed` _charactermovement) _cskillinfo_speedupratio_2) _charactermovement)
  (bind _returnvalue (`KismetSystemLibrary.K2_SetTimer` null (`local.CSkillTickFunctionName`) 0.003333 true true))
  (set `self.CSkillTickHandler` _returnvalue)
  (set `self.CSkillInfo` (make `/Game/ProjectSD/Blueprints/Character/Player/PlayerSkill/EachSkillStructure/BunnyCSkillInfo` _cskillinfo_isaction _cskillinfo_isactioncooltime _cskillinfo_currentcooltime _cskillinfo_maxcooltime _cskillinfo_mentalityconsumption true _cskillinfo_mentalityconsumptionperseconds _cskillinfo_speedupratio _cskillinfo_gainelectricforceratio)))

(fn `CSkillTick`
  (locals (UltimateGainElectricForceRatio :type "Float (double-precision)" :default 0.06) (MoveGap :type "Float (double-precision)" :default 100.0))
  (bind _movegap (`local.MoveGap`))
  (bind (_cskillinfo_isaction _cskillinfo_isactioncooltime _cskillinfo_currentcooltime _cskillinfo_maxcooltime _cskillinfo_mentalityconsumption _cskillinfo_onoff _cskillinfo_mentalityconsumptionperseconds _cskillinfo_speedupratio _cskillinfo_gainelectricforceratio) (break `/Game/ProjectSD/Blueprints/Character/Player/PlayerSkill/EachSkillStructure/BunnyCSkillInfo` (`self.CSkillInfo`)))
  (bind _maxelectricforce (`self.MaxElectricForce`))
  (bind (_cskillinfo_isaction_2 _cskillinfo_isactioncooltime_2 _cskillinfo_currentcooltime_2 _cskillinfo_maxcooltime_2 _cskillinfo_mentalityconsumption_2 _cskillinfo_onoff_2 _cskillinfo_mentalityconsumptionperseconds_2) (break `/Game/ProjectSD/Blueprints/Character/Player/PlayerSkill/EachSkillStructure/BunnyCSkillInfo` (`self.CSkillInfo`)))
  (bind _cskillmovedistance (`self.CSkillMoveDistance`))
  (bind _isremovable (`/Game/ProjectSD/Blueprints/Character/Player/BP_PlayerCharacter.RemoveMentality` (`self.TargetCharacter`) (* (`GameplayStatics.GetWorldDeltaSeconds`) _cskillinfo_mentalityconsumptionperseconds_2)))
  (if _isremovable
    ; 이동 거리 갱신
    (set `self.CSkillMoveDistance` (+ (`self.CSkillMoveDistance`) (`self.GetLastMoveDistance`)))
    ; 이동 거리에 따라 전기력 충전
    (if (>= _cskillmovedistance _movegap)
      (set `self.CSkillMoveDistance` (- _cskillmovedistance _movegap))
      (set `self.CurrentElectricForce` (`KismetMathLibrary.FClamp` (+ (`self.CurrentElectricForce`) (* _maxelectricforce _cskillinfo_gainelectricforceratio)) 0.0 _maxelectricforce)))
    (else
      (`self.CSkillOff`))))

(fn `DoOnLanded`
  (locals (WaveRadius :type "Float (double-precision)" :default 400.0) (WaveHeight :type "Float (double-precision)" :default -0.4) (Query :type "Array of EObjectTypeQuery Enum") (NewLocalVar :type "Array of Actor Object Reference") (TargetEnemyNum :type Integer :default 0) (TargetEnumeyNumMax :type Integer :default 6) (WaveDamage :type Integer :default 10) (TargetEnemy :type "Array of Actor Object Reference"))
  (bind _targetcharacter (`self.TargetCharacter`))
  (bind _targetcharacter_2 (`self.TargetCharacter`))
  (bind (_distance _returnvalue) (`GameplayStatics.FindNearestActor` (`Actor.K2_GetActorLocation` _targetcharacter_2) (`local.TargetEnemy`)))
  (if (`/Game/ProjectSD/Blueprints/Character/Player/BP_PlayerCharacter.IsJumpCompleted` _targetcharacter)
    (`KismetSystemLibrary.PrintString` "Attack Wave!!!" true true (struct :`R` 1.0 :`G` 0.095359 :`A` 1.0))
    (bind _output_get (set `local.WaveHeight` (* (`CapsuleComponent.CapsuleHalfHeight` (`Character.CapsuleComponent` _targetcharacter)) 2.0)))
    (bind _outactors (`KismetSystemLibrary.CapsuleOverlapActors` (`Actor.K2_GetActorLocation` _targetcharacter) (`local.WaveRadius`) _output_get (`local.Query`) "/Game/ProjectSD/Blueprints/Character/Enemy/Base/BP_EnemyBase.BP_EnemyBase_C"))
    (`GameplayStatics.SpawnEmitterAttached` "/Game/StarterContent/Particles/P_Explosion.P_Explosion" (`Character.Mesh` (`self.TargetCharacter`)))
    (set `local.TargetEnemy` _outactors)
    (while (not (or (>= (`local.TargetEnemyNum`) (`local.TargetEnumeyNumMax`)) (<= (`KismetArrayLibrary.Array_Length` (`local.TargetEnemy`)) 0)))
      (`GameplayStatics.ApplyDamage` _returnvalue (* (`/Game/ProjectSD/Blueprints/Character/Player/BP_PlayerCharacter.AttackDamage` _targetcharacter_2) (`local.WaveDamage`)) null _targetcharacter_2)
      (`KismetArrayLibrary.Array_RemoveItem` (`local.TargetEnemy`) _returnvalue)
      (set `local.TargetEnemyNum` (+ (`local.TargetEnemyNum`) 1)))
    (return)))

(fn `DoOnLandedInterface`
  (`self.DoOnLanded`))

(fn `GetLastMoveDistance`
  (returns (LastMoveDistance :type "Float (double-precision)"))
  (return (* (`KismetMathLibrary.VSize` (`Actor.GetVelocity` (`self.TargetCharacter`))) (`GameplayStatics.GetWorldDeltaSeconds`))))

(fn `PassiveTick`
  (params (DeltaTime :type "Float (double-precision)"))
  (locals (MoveGap :type "Float (double-precision)" :default 100.0))
  (bind _movegap (`local.MoveGap`))
  (bind _maxelectricforce (`self.MaxElectricForce`))
  (bind _passivemovedistance (`self.PassiveMoveDistance`))
  (if (`|EnumInequality` (`/Game/ProjectSD/Blueprints/Character/Player/BP_PlayerCharacter.CurrentHookStatus` (`self.TargetCharacter`)) "NewEnumerator2")
    (`|ExecutionSequence`
      (:`then_0`
        ; 이동 거리 갱신
        (set `self.PassiveMoveDistance` (+ (`self.PassiveMoveDistance`) (`self.GetLastMoveDistance`))))
      (:`then_1`
        ; 이동 거리에 따라 전기력 충전
        (if (>= _passivemovedistance _movegap)
          (set `self.PassiveMoveDistance` (- _passivemovedistance _movegap))
          (set `self.CurrentElectricForce` (`KismetMathLibrary.FClamp` (+ (`self.CurrentElectricForce`) (* _maxelectricforce (`self.GainElectricForceRatio`))) 0.0 _maxelectricforce))))
      (:`then_2`
        (`|ExecutionSequence`
          (:`then_0`
            ; 움직임이 없다면 일정간격으로 전기력 감소
            (if (<= (`self.GetLastMoveDistance`) 0.0)
              (bind _output_get (set `self.CurrentMoveWaitingTime` (+ (`self.CurrentMoveWaitingTime`) DeltaTime)))
              (if (>= _output_get (`self.MaxMoveWaitingTime`))
                (`self.ConsumeElectricForcePerSecond` (* (`self.MaxElectricForce`) (`self.LossElectricForceRatio`)) (`local.DeltaTime`))
                (set `self.CurrentMoveWaitingTime` (`self.MaxMoveWaitingTime`)))
              (else
                (set `self.CurrentMoveWaitingTime` 0.0))))
          (:`then_1`
            ; UI 갱신
            (`/Game/ProjectSD/Blueprints/Character/Player/PlayerSkill/PlayerSkillUI/BP_BunnySkillPassive.SetElectricForceGage` (`self.ElectricForceWidget`) (`self.CurrentElectricForce`) (`self.MaxElectricForce`) :!label _label)))))
    (else
      (goto _label))))

(fn `TurnOffAllIsAction`
  (bind (_cskillinfo_isaction _cskillinfo_isactioncooltime _cskillinfo_currentcooltime _cskillinfo_maxcooltime _cskillinfo_mentalityconsumption _cskillinfo_onoff _cskillinfo_mentalityconsumptionperseconds _cskillinfo_speedupratio _cskillinfo_gainelectricforceratio) (break `/Game/ProjectSD/Blueprints/Character/Player/PlayerSkill/EachSkillStructure/BunnyCSkillInfo` (`self.CSkillInfo`)))
  (set `self.CSkillInfo` (make `/Game/ProjectSD/Blueprints/Character/Player/PlayerSkill/EachSkillStructure/BunnyCSkillInfo` false _cskillinfo_isactioncooltime _cskillinfo_currentcooltime _cskillinfo_maxcooltime _cskillinfo_mentalityconsumption _cskillinfo_onoff _cskillinfo_mentalityconsumptionperseconds _cskillinfo_speedupratio _cskillinfo_gainelectricforceratio)))

(fn `ZSkillOff`
  (bind _targetcharacter (`self.TargetCharacter`))
  (bind (_zskillinfo_isaction _zskillinfo_isactioncooltime _zskillinfo_currentcooltime _zskillinfo_maxcooltime _zskillinfo_electricforceconsumptionpersecond _zskillinfo_onoff) (break `/Game/ProjectSD/Blueprints/Character/Player/PlayerSkill/EachSkillStructure/BunnyZSkillInfoBase` (`self.ZSkillInfo`)))
  (if _zskillinfo_onoff
    (if (`KismetSystemLibrary.K2_IsValidTimerHandle` (`self.ZSkillOffTickHandler`))
      (`KismetSystemLibrary.PrintString` "반복적 off 실행")
      (else
        (`/Game/ProjectSD/Blueprints/Character/Player/PlayerSkill/EachSkillActor/BP_ZSkillBeamActor.TurnOff` (`self.ZSkillBeamActor`))
        (set `CharacterMovementComponent.MaxWalkSpeed` (`/Game/ProjectSD/Blueprints/Character/Player/BP_PlayerCharacter.DefaultMaxSpeed` _targetcharacter) (`Character.CharacterMovement` _targetcharacter))
        (`KismetSystemLibrary.K2_ClearAndInvalidateTimerHandle` (`self.ZSkillTickHandler`))
        (bind _returnvalue (`KismetSystemLibrary.K2_SetTimer` null "ZSkillOffTick" 0.003333 true true))
        (set `self.ZSkillOffTickHandler` _returnvalue)
        (bind _returnvalue_2 (`KismetSystemLibrary.K2_SetTimer` null "ZSkillRealOff" 0.003333 true true))
        (set `self.ZSkillRealOffHandler` _returnvalue_2)
        (`GameplayStatics.SpawnSound2D` "/Game/Resources/Sounds/Player/Skill4/PC_Se_Bunny_Active4_Beam_Release.PC_Se_Bunny_Active4_Beam_Release" 1.0 1.0 0.0 null)
        (`AudioComponent.Stop` (`self.BeamSound`))
        (set `/Game/ProjectSD/Blueprints/Character/Player/BP_PlayerCharacter.Skill4Status` "NewEnumerator3" (`self.TargetCharacter`))))))

(fn `ZSkillOffTick`
  (locals (MaxTime :type "Float (double-precision)" :default 0.5))
  (bind (_zskillinfo_isaction _zskillinfo_isactioncooltime _zskillinfo_currentcooltime _zskillinfo_maxcooltime _zskillinfo_electricforceconsumptionpersecond) (break `/Game/ProjectSD/Blueprints/Character/Player/PlayerSkill/EachSkillStructure/BunnyZSkillInfoBase` (`self.ZSkillInfo`)))
  (if (`self.IsZSkillTickRunning`)
    (`self.ConsumeElectricForcePerSecond` _zskillinfo_electricforceconsumptionpersecond (`GameplayStatics.GetWorldDeltaSeconds`)))
  (set `self.CurrentZSkillOffTickTime` (+ (`GameplayStatics.GetWorldDeltaSeconds`) (`self.CurrentZSkillOffTickTime`)))
  (bind _iscompleted (`self.CalculateCoolTime` (`GameplayStatics.GetWorldDeltaSeconds`) (`self.CurrentZSkillOffTickTime`) (`local.MaxTime`)))
  (if _iscompleted
    (set `self.CurrentZSkillOffTickTime` 0.0)
    (`KismetSystemLibrary.K2_ClearAndInvalidateTimerHandle` (`self.ZSkillOffTickHandler`))))

(fn `ZSkillOn`
  (locals (StartSkillDelay :type "Float (double-precision)" :default 0.75) (ZSkillTickFunctionName :type String :default "ZSkillTick"))
  (bind _targetcharacter (`self.TargetCharacter`))
  (bind (_zskillinfo_isaction _zskillinfo_isactioncooltime _zskillinfo_currentcooltime _zskillinfo_maxcooltime _zskillinfo_electricforceconsumptionpersecond _zskillinfo_onoff _zskillinfo_speeddownratio) (break `/Game/ProjectSD/Blueprints/Character/Player/PlayerSkill/EachSkillStructure/BunnyZSkillInfoBase` (`self.ZSkillInfo`)))
  (bind _targetcharacter_2 (`self.TargetCharacter`))
  (bind _startskilldelay (`local.StartSkillDelay`))
  (bind (_zskillinfo_isaction_2 _zskillinfo_isactioncooltime_2 _zskillinfo_currentcooltime_2 _zskillinfo_maxcooltime_2 _zskillinfo_electricforceconsumptionpersecond_2 _zskillinfo_onoff_2 _zskillinfo_speeddownratio_2 _zskillinfo_currentticktime) (break `/Game/ProjectSD/Blueprints/Character/Player/PlayerSkill/EachSkillStructure/BunnyZSkillInfoBase` (`self.ZSkillInfo`)))
  (bind _charactermovement (`Character.CharacterMovement` _targetcharacter))
  (set `/Game/ProjectSD/Blueprints/Character/Player/BP_PlayerCharacter.IsHookableSkill` false _targetcharacter)
  (`self.CSkillOff`)
  (`KismetSystemLibrary.K2_SetTimer` null "ZSkillStartTick" _startskilldelay)
  (set `CharacterMovementComponent.MaxWalkSpeed` (* (`CharacterMovementComponent.MaxWalkSpeed` _charactermovement) _zskillinfo_speeddownratio) _charactermovement)
  (bind _returnvalue (`KismetSystemLibrary.K2_SetTimer` null (`local.ZSkillTickFunctionName`) 0.003333 true true _startskilldelay))
  (set `self.ZSkillTickHandler` _returnvalue)
  (set `self.ZSkillInfo` (make `/Game/ProjectSD/Blueprints/Character/Player/PlayerSkill/EachSkillStructure/BunnyZSkillInfoBase` _zskillinfo_isaction_2 _zskillinfo_isactioncooltime_2 _zskillinfo_currentcooltime_2 _zskillinfo_maxcooltime_2 _zskillinfo_electricforceconsumptionpersecond_2 true _zskillinfo_speeddownratio_2 _zskillinfo_currentticktime))
  (set `/Game/ProjectSD/Blueprints/Character/Player/BP_PlayerCharacter.PlayerStatus` "NewEnumerator5" _targetcharacter_2)
  (`/Game/ProjectSD/Blueprints/Character/Player/PlayerUI/WB_PlayerCharacterTotal.TurnOffGunAimUI` (`/Game/ProjectSD/Blueprints/Character/Player/BP_PlayerCharacter.UITotal` _targetcharacter_2))
  (`GameplayStatics.SpawnSound2D` "/Game/Resources/Sounds/Player/Skill4/PC_Se_Bunny_Active4_Start.PC_Se_Bunny_Active4_Start" 1.0 1.0 0.0 null)
  (set `/Game/ProjectSD/Blueprints/Character/Player/BP_PlayerCharacter.Skill4Status` "NewEnumerator1" (`self.TargetCharacter`)))

(fn `ZSkillRealOff`
  (bind (_zskillinfo_isaction _zskillinfo_isactioncooltime _zskillinfo_currentcooltime _zskillinfo_maxcooltime _zskillinfo_electricforceconsumptionpersecond _zskillinfo_onoff _zskillinfo_speeddownratio _zskillinfo_currentticktime _zskillinfo_attackrank) (break `/Game/ProjectSD/Blueprints/Character/Player/PlayerSkill/EachSkillStructure/BunnyZSkillInfoBase` (`self.ZSkillInfo`)))
  (bind _targetcharacter (`self.TargetCharacter`))
  (if (not (`KismetSystemLibrary.K2_IsValidTimerHandle` (`self.ZSkillOffTickHandler`)))
    (set `self.ZSkillInfo` (make `/Game/ProjectSD/Blueprints/Character/Player/PlayerSkill/EachSkillStructure/BunnyZSkillInfoBase` _zskillinfo_isaction false 0.0 _zskillinfo_maxcooltime _zskillinfo_electricforceconsumptionpersecond false _zskillinfo_speeddownratio _zskillinfo_currentticktime _zskillinfo_attackrank))
    (`KismetSystemLibrary.K2_ClearAndInvalidateTimerHandle` (`self.ZSkillRealOffHandler`))
    (set `self.IsZSkillTickRunning` false)
    (set `/Game/ProjectSD/Blueprints/Character/Player/BP_PlayerCharacter.IsHookableSkill` true (`self.TargetCharacter`))
    (set `/Game/ProjectSD/Blueprints/Character/Player/BP_PlayerCharacter.PlayerStatus` "NewEnumerator4" _targetcharacter)
    (`/Game/ProjectSD/Blueprints/Character/Player/PlayerUI/WB_PlayerCharacterTotal.TurnOnGunAimUI` (`/Game/ProjectSD/Blueprints/Character/Player/BP_PlayerCharacter.UITotal` _targetcharacter))
    (set `/Game/ProjectSD/Blueprints/Character/Player/BP_PlayerCharacter.Skill4Status` "NewEnumerator0" (`self.TargetCharacter`))))

(fn `ZSkillStartTick`
  (`GameplayStatics.SpawnSound2D` "/Game/Resources/Sounds/Player/Skill4/PC_Se_Bunny_Active4_Beam_Start.PC_Se_Bunny_Active4_Beam_Start" 1.0 1.0 0.0 null)
  (`AudioComponent.Play` (`self.BeamSound`) 0.0)
  (set `/Game/ProjectSD/Blueprints/Character/Player/BP_PlayerCharacter.Skill4Status` "NewEnumerator2" (`self.TargetCharacter`)))

(fn `ZSkillTick`
  (locals (TemptTickTime :type "Float (double-precision)") (TemptRank :type Integer) (Time1to2 :type "Float (double-precision)" :default 1.1) (Time2to3 :type "Float (double-precision)" :default 1.1) (DefaultDamageRatio :type "Float (double-precision)" :default 0.2) (Rank2DamageRatio :type "Float (double-precision)" :default 2.0) (Rank3DamageRatio :type "Float (double-precision)" :default 4.0) (CurrentDamage :type "Float (double-precision)") (TargetPoint :type "Vector Structure") (FinalDistance :type "Float (double-precision)") (NewLocalVar_0 :type "Array of Actor Object Reference"))
  (bind (_zskillinfo_isaction _zskillinfo_isactioncooltime _zskillinfo_currentcooltime _zskillinfo_maxcooltime _zskillinfo_electricforceconsumptionpersecond) (break `/Game/ProjectSD/Blueprints/Character/Player/PlayerSkill/EachSkillStructure/BunnyZSkillInfoBase` (`self.ZSkillInfo`)))
  (bind (_zskillinfo_isaction_2 _zskillinfo_isactioncooltime_2 _zskillinfo_currentcooltime_2 _zskillinfo_maxcooltime_2 _zskillinfo_electricforceconsumptionpersecond_2 _zskillinfo_onoff _zskillinfo_speeddownratio _zskillinfo_currentticktime) (break `/Game/ProjectSD/Blueprints/Character/Player/PlayerSkill/EachSkillStructure/BunnyZSkillInfoBase` (`self.ZSkillInfo`)))
  (bind _zskillbeamactor (`self.ZSkillBeamActor`))
  (bind _time1to2 (`local.Time1to2`))
  (bind (_zskillinfo_isaction_3 _zskillinfo_isactioncooltime_3 _zskillinfo_currentcooltime_3 _zskillinfo_maxcooltime_3 _zskillinfo_electricforceconsumptionpersecond_3 _zskillinfo_onoff_2 _zskillinfo_speeddownratio_2 _zskillinfo_currentticktime_2 _zskillinfo_attackrank) (break `/Game/ProjectSD/Blueprints/Character/Player/PlayerSkill/EachSkillStructure/BunnyZSkillInfoBase` (`self.ZSkillInfo`)))
  (bind _hookhand (`/Game/ProjectSD/Blueprints/Character/Player/BP_PlayerCharacter.HookHand` (`self.TargetCharacter`)))
  (bind _returnvalue (`SceneComponent.K2_GetComponentLocation` (`/Game/ProjectSD/Blueprints/Character/Player/BP_PlayerCharacter.Camera` (`self.TargetCharacter`))))
  (bind _returnvalue_2 (* (`local.DefaultDamageRatio`) (`/Game/ProjectSD/Blueprints/Character/Player/BP_PlayerCharacter.AttackDamage` (`self.TargetCharacter`))))
  (bind _returnvalue_3 (+ _returnvalue (* (`KismetMathLibrary.GetForwardVector` (`Controller.GetDesiredRotation` (`GameplayStatics.GetPlayerController` 0))) 2000)))
  (set `self.IsZSkillTickRunning` true)
  (bind _iscompleted (`self.ConsumeElectricForcePerSecond` _zskillinfo_electricforceconsumptionpersecond (`GameplayStatics.GetWorldDeltaSeconds`)))
  (if _iscompleted
    (bind _output_get (set `local.TemptTickTime` (+ (`GameplayStatics.GetWorldDeltaSeconds`) _zskillinfo_currentticktime)))
    (if (>= _output_get (+ (`local.Time2to3`) _time1to2))
      (set `local.TemptRank` 3)
      (elif (>= _output_get _time1to2)
        (set `local.TemptRank` 2)
        (else
          (set `local.TemptRank` 1))))
    (set `self.ZSkillInfo` (make `/Game/ProjectSD/Blueprints/Character/Player/PlayerSkill/EachSkillStructure/BunnyZSkillInfoBase` _zskillinfo_isaction_2 _zskillinfo_isactioncooltime_2 _zskillinfo_currentcooltime_2 _zskillinfo_maxcooltime_2 _zskillinfo_electricforceconsumptionpersecond_2 _zskillinfo_onoff _zskillinfo_speeddownratio (`local.TemptTickTime`) (`local.TemptRank`)))
    (switch `int` _zskillinfo_attackrank
      (:`1`
        (set `local.CurrentDamage` _returnvalue_2))
      (:`2`
        (set `local.CurrentDamage` (* _returnvalue_2 (`local.Rank2DamageRatio`))))
      (:`3`
        (set `local.CurrentDamage` (* _returnvalue_2 (`local.Rank3DamageRatio`)))))
    (bind (_outhit _returnvalue_4) (`KismetSystemLibrary.LineTraceSingle` :`Start` _returnvalue :`End` _returnvalue_3 :`TraceChannel` "TraceTypeQuery1" :`DrawDebugType` "ForOneFrame" :`TraceColor` (struct :`G` 1.0 :`B` 0.408086 :`A` 1.0)))
    (if _returnvalue_4
      (set `local.TargetPoint` (`.Location` (`GameplayStatics.BreakHitResult` _outhit)))
      (else
        (set `local.TargetPoint` _returnvalue_3)))
    (bind (_outhit_2 _returnvalue_5) (`KismetSystemLibrary.LineTraceSingle` :`Start` (`/Game/ProjectSD/Blueprints/Character/Player/BP_PlayerCharacter.HookHand` (`self.TargetCharacter`)) :`End` (`local.TargetPoint`) :`TraceChannel` "TraceTypeQuery3" :`DrawDebugType` "ForOneFrame" :`TraceColor` (struct :`A` 1.0) :`TraceHitColor` (struct :`A` 1.0)))
    (if _returnvalue_5
      (bind (_bblockinghit _binitialoverlap _time _distance _location _impactpoint _normal _impactnormal _physmat _hitactor) (`GameplayStatics.BreakHitResult` _outhit_2))
      (set `local.TargetPoint` _location)
      (set `local.FinalDistance` _distance)
      (else
        (set `local.FinalDistance` (`KismetMathLibrary.VSize` (- (`local.TargetPoint`) _hookhand)))))
    (bind _outhits (`KismetSystemLibrary.SphereTraceMulti` :`Start` _hookhand :`End` (`local.TargetPoint`) :`Radius` 10.0 :`TraceChannel` "TraceTypeQuery4" :`DrawDebugType` "ForOneFrame" :`TraceColor` (struct :`R` 0.207866 :`G` 0.088914 :`B` 1.0 :`A` 1.0) :`TraceHitColor` (struct :`R` 0.089732 :`G` 0.072215 :`B` 1.0 :`A` 1.0)))
    (for _array_element _outhits
      (bind (_bblockinghit_2 _binitialoverlap_2 _time_2 _distance_2 _location_2 _impactpoint_2 _normal_2 _impactnormal_2 _physmat_2 _hitactor_2 _hitcomponent _hitbonename _bonename _hititem _elementindex _faceindex _tracestart _traceend) (`GameplayStatics.BreakHitResult` _array_element))
      (`GameplayStatics.ApplyPointDamage` _hitactor_2 (`local.CurrentDamage`) (- _traceend _tracestart) _array_element))
    (`/Game/ProjectSD/Blueprints/Character/Player/PlayerSkill/EachSkillActor/BP_ZSkillBeamActor.TurnOn` _zskillbeamactor)
    (`/Game/ProjectSD/Blueprints/Character/Player/PlayerSkill/EachSkillActor/BP_ZSkillBeamActor.SetEndPoint` _zskillbeamactor (`local.TargetPoint`))
    (else
      (`self.ZSkillOff`))))