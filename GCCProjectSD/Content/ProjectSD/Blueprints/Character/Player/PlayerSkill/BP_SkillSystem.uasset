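; BP_SkillSystem is the player character's skill system, with Q, C, V and Z skill actions that are currently stubs printing debug strings.
; On BeginPlay it casts its outer object to BP_PlayerCharacter and stores it as TargetCharacter.
; A CalculateCoolTime helper adds delta time to a cooldown, clamps it at the maximum and reports completion, though nothing in this file calls it.
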(event `self.ReceiveBeginPlay`
  (bind _asbp_player_character (cast `/Game/ProjectSD/Blueprints/Character/Player/BP_PlayerCharacter` (`KismetSystemLibrary.GetOuterObject` self)))
  (set `self.TargetCharacter` _asbp_player_character))

(fn `ActionCSkill`
  (`KismetSystemLibrary.PrintString` "UseC"))

(fn `ActionQSkill`
  (`KismetSystemLibrary.PrintString` "UseQ"))

(fn `ActionVSkill`
  (`KismetSystemLibrary.PrintString` "UseV"))

(fn `ActionZSkill`
  (`KismetSystemLibrary.PrintString` "UseZ"))

(fn `CalculateCoolTime`
  (params (DeltaTime :type "Float (double-precision)") (CurrentCoolTime :type "Float (double-precision)") (MaxCoolTime :type "Float (double-precision)"))
  (returns (IsCompleted :type Boolean) (NextCoolTime :type "Float (double-precision)"))
  (locals (CurrentCoolTimeTempt :type "Float (double-precision)") (IsCompletedTempt :type Boolean))
  (bind _output_get (set `local.CurrentCoolTimeTempt` (+ DeltaTime CurrentCoolTime)))
  (if (>= _output_get MaxCoolTime)
    (set `local.CurrentCoolTimeTempt` (`local.MaxCoolTime`))
    (set `local.IsCompletedTempt` true))
  (return (`local.IsCompletedTempt`) (`local.CurrentCoolTimeTempt`)))