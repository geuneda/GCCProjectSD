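; Beam visual actor for the player's Z skill, built around a Niagara effect and owned by the player character.
; On BeginPlay it caches the owning player character as its target character.
; TurnOn and TurnOff toggle the effect's visibility, and SetEndPoint writes a supplied location to the Niagara beam-end parameter.
; It applies no hits itself: an enemy capsule trace is left unconnected.
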(event `self.ReceiveBeginPlay`
  (bind _asbp_player_character (cast `/Game/ProjectSD/Blueprints/Character/Player/BP_PlayerCharacter` (`self.GetOwner`)))
  (set `self.TargetCharacter` _asbp_player_character))

(fn `SetEndPoint`
  (params (EndPointLocation :type "Vector Structure"))
  (`NiagaraComponent.SetVariableVec3` (`self.Niagara`) "User.Beam_End" EndPointLocation))

(fn `TurnOff`
  (`SceneComponent.SetVisibility` (`self.Niagara`) false false))

(fn `TurnOn`
  (`SceneComponent.SetVisibility` (`self.Niagara`) true false))

(fn `UserConstructionScript`)