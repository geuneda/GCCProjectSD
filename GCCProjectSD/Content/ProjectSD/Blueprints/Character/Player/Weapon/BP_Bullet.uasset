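; BP_Bullet is a projectile fired by the player character that damages whatever it hits.
; On hit, it casts its owner to BP_PlayerCharacter and deals point damage randomized around that player's AttackDamage, rounded down.
; It then spawns a small explosion, plays an impact sound and destroys itself, or prints an error if the owner cast fails.
; A forward line trace and other leftover damage nodes are unconnected.
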(event `self.ReceiveHit`
  (params (MyComp :type "PrimitiveComponent Object Reference") (Other :type "Actor Object Reference") (OtherComp :type "PrimitiveComponent Object Reference") (bSelfMoved :type Boolean) (HitLocation :type "Vector Structure") (HitNormal :type "Vector Structure") (NormalImpulse :type "Vector Structure") (Hit :type "HitResult Structure (by ref)"))
  (bind (_hitscan_bblockinghit _hitscan_binitialoverlap _hitscan_time _hitscan_distance _hitscan_location _hitscan_impactpoint _hitscan_normal _hitscan_impactnormal _hitscan_physmat _hitscan_hitactor _hitscan_hitcomponent _hitscan_hitbonename _hitscan_bonename _hitscan_hititem _hitscan_elementindex _hitscan_faceindex _hitscan_tracestart _hitscan_traceend) (`GameplayStatics.BreakHitResult` (`self.HitScan`)))
  (bind (_hitscan_bblockinghit_2 _hitscan_binitialoverlap_2 _hitscan_time_2 _hitscan_distance_2 _hitscan_location_2 _hitscan_impactpoint_2 _hitscan_normal_2 _hitscan_impactnormal_2 _hitscan_physmat_2 _hitscan_hitactor_2 _hitscan_hitcomponent_2) (`GameplayStatics.BreakHitResult` (`self.HitScan`)))
  (set `self.HitScan` Hit)
  (bind _asbp_player_character (cast `/Game/ProjectSD/Blueprints/Character/Player/BP_PlayerCharacter` (`self.GetOwner`))
    (:`then`
      (if (== _hitscan_hitactor Other)
        (bind _attackdamage (`/Game/ProjectSD/Blueprints/Character/Player/BP_PlayerCharacter.AttackDamage` _asbp_player_character))
        (`GameplayStatics.ApplyPointDamage` Other (`KismetMathLibrary.Conv_IntToDouble` (`KismetMathLibrary.FFloor` (`KismetMathLibrary.RandomFloatInRange` (`KismetMathLibrary.FClamp` (- _attackdamage 5.0) 1.0 _attackdamage) (+ _attackdamage 5.0)))) (- _hitscan_traceend _hitscan_tracestart) (`self.HitScan`))
        (`GameplayStatics.SpawnEmitterAttached` "/Game/StarterContent/Particles/P_Explosion.P_Explosion" _hitscan_hitcomponent_2 "None" _hitscan_location_2 (struct) (0.1 0.1 0.1) "KeepWorldPosition")
        (`GameplayStatics.PlaySoundAtLocation` "/Game/ProjectSD/Blueprints/Character/Player/Weapon/Hit_Generic_5-1.Hit_Generic_5-1" _hitscan_location_2 (struct) 1.0 1.0 0.0 "/USDCore/USDDefaultAttenuation.USDDefaultAttenuation" null null null)
        (`self.K2_DestroyActor`)))
    (:`CastFailed`
      (`KismetSystemLibrary.PrintString` "Error!!!" true true (struct :`R` 1.0 :`B` 0.775604 :`A` 1.0) 10.0))))

(event `self.ReceiveActorBeginOverlap`
  (params (OtherActor :type "Actor Object Reference")))

(event `self.ReceiveTick`
  (params (DeltaSeconds :type "Float (single-precision)")))

(fn `UserConstructionScript`)