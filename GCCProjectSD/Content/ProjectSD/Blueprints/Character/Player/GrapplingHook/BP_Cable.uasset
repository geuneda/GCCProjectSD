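; Grappling hook cable actor that links the player's hand to a fired BP_CableHook projectile.
; On BeginPlay it spawns the hook toward the aim point, or along control rotation when no shot is valid, destroying itself shortly after in that case.
; The cable start follows the hand each tick and its end attaches to the hook using a scale-corrected offset.
; Hook hits trigger StartGrapplingHook on the player; destroying the cable destroys the hook.
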(event `self.ReceiveBeginPlay`
  (bind _ownerplayer (`self.OwnerPlayer`))
  (bind _ownerplayer_2 (`self.OwnerPlayer`))
  (bind _hookhand (`/Game/ProjectSD/Blueprints/Character/Player/BP_PlayerCharacter.HookHand` _ownerplayer))
  (bind _asbp_player_character (cast `/Game/ProjectSD/Blueprints/Character/Player/BP_PlayerCharacter` (`self.GetOwner`)))
  (bind _output_get (set `self.OwnerPlayer` _asbp_player_character))
  (if (`/Game/ProjectSD/Blueprints/Character/Player/BP_PlayerCharacter.IsHookShootable` _output_get)
    (bind _returnvalue (`|SpawnActorFromClass` "/Game/ProjectSD/Blueprints/Character/Player/GrapplingHook/BP_CableHook.BP_CableHook_C" (`KismetMathLibrary.MakeTransform` _hookhand (`KismetMathLibrary.FindLookAtRotation` _hookhand (`/Game/ProjectSD/Blueprints/Character/Player/BP_PlayerCharacter.ShootEndPoint` _ownerplayer))) "Undefined" "MultiplyWithRoot" null null))
    (bind _output_get_2 (set `self.TargetCableHook` _returnvalue))
    (else
      (bind _returnvalue_2 (`|SpawnActorFromClass` "/Game/ProjectSD/Blueprints/Character/Player/GrapplingHook/BP_CableHook.BP_CableHook_C" (`KismetMathLibrary.MakeTransform` (`/Game/ProjectSD/Blueprints/Character/Player/BP_PlayerCharacter.HookHand` _ownerplayer_2) (`Pawn.GetControlRotation` _ownerplayer_2)) "Undefined" "MultiplyWithRoot" null null))
      (set `self.TargetCableHook` _returnvalue_2)))
  (add `/Game/ProjectSD/Blueprints/Character/Player/GrapplingHook/BP_CableHook.OnComponentHit` _output_get_2 (delegate `EventHitHook`))
  (bind _newparam (`/Game/ProjectSD/Blueprints/Character/Player/GrapplingHook/BP_CableHook.GetCollision` _output_get_2))
  (`self.SetHitEndPoint` _newparam (`SceneComponent.K2_GetComponentLocation` _newparam))
  (if (not (`/Game/ProjectSD/Blueprints/Character/Player/BP_PlayerCharacter.IsHookShootable` (`self.OwnerPlayer`)))
    (`KismetSystemLibrary.Delay` 0.2)
    (`self.K2_DestroyActor`)))

(event `EventHitHook`
  (params (HitComponent :type "PrimitiveComponent Object Reference") (OtherActor :type "Actor Object Reference") (OtherComp :type "PrimitiveComponent Object Reference") (NormalImpulse :type "Vector Structure") (Hit :type "HitResult Structure"))
  (`self.LaunchPlayer` HitComponent (`SceneComponent.K2_GetComponentLocation` HitComponent) (`.Normal` (`GameplayStatics.BreakHitResult` Hit))))

(event `self.ReceiveTick`
  (params (DeltaSeconds :type "Float (single-precision)"))
  (`self.K2_SetActorLocation` (`/Game/ProjectSD/Blueprints/Character/Player/BP_PlayerCharacter.HookHand` (`self.OwnerPlayer`))))

(event `self.ReceiveDestroyed`
  (`self.K2_DestroyActor` (`self.TargetCableHook`)))

(fn `LaunchPlayer`
  (params (HitComponent :type "PrimitiveComponent Object Reference") (HitWorldLocation :type "Vector Structure") (HitNormal :type "Vector Structure"))
  (`self.SetHitEndPoint` HitComponent HitWorldLocation)
  (`/Game/ProjectSD/Blueprints/Character/Player/BP_PlayerCharacter.StartGrapplingHook` (`self.OwnerPlayer`) HitComponent HitWorldLocation HitNormal))

(fn `SetHitEndPoint`
  (params (HitComponent :type "SceneComponent Object Reference") (HitWorldLocation :type "Vector Structure"))
  (locals (Offset :type "Vector Structure"))
  (bind (_returnvalue_x _returnvalue_y _returnvalue_z) (`KismetMathLibrary.BreakVector` (`SceneComponent.K2_GetComponentScale` (`local.HitComponent`))))
  (`CableComponent.SetAttachEndToComponent` (`self.CableComponent`) HitComponent "None")
  (bind _output_get (set `local.Offset` (- (`local.HitWorldLocation`) (`SceneComponent.K2_GetComponentLocation` (`local.HitComponent`)))))
  (bind _output_get_2 (set `local.Offset` (`KismetMathLibrary.MakeVector` (/ (.x _output_get) _returnvalue_x) (/ (.y _output_get) _returnvalue_y) (/ (.z _output_get) _returnvalue_z))))
  (set `CableComponent.EndLocation` _output_get_2 (`self.CableComponent`)))

(fn `UserConstructionScript`)