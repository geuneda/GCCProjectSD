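; Base player character Blueprint providing mouse-look camera, movement and a double jump.
; Mouse input applies yaw to the Aim component and clamped pitch to the SpringArm, separating heading from camera tilt.
; Tick moves the actor relative to Aim with swept SetActorLocation rather than movement input, turning the mesh to Aim's forward while moving.
; Space uses a jump counter: Jump first, then LaunchCharacter at the JumpZVelocity cached on BeginPlay.
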(event `InputVectorAxis|Mouse2D`
  (params (AxisValue :type "Vector Structure"))
  (bind (_returnvalue_x _returnvalue_y) (`KismetMathLibrary.BreakVector` (+ (`KismetMathLibrary.MakeVector` (.x (* AxisValue (`GameplayStatics.GetWorldDeltaSeconds`) (`self.Sensitive`))) (.y (* AxisValue (`GameplayStatics.GetWorldDeltaSeconds`) (`self.Sensitive`)))) (`self.CurrentCameraRelativeRot`))))
  ; 마우스 입력에 따른 카메라 회전
  (bind _output_get (set `self.CurrentCameraRelativeRot` (`KismetMathLibrary.MakeVector` _returnvalue_x (`KismetMathLibrary.FClamp` _returnvalue_y (* (`self.PitchMaxAbs`) -1.0) (`self.PitchMaxAbs`)))))
  (`SceneComponent.K2_SetRelativeRotation` (`self.Aim`) (`KismetMathLibrary.MakeRotator` 0.0 0.0 (.x _output_get)) false false)
  (`SceneComponent.K2_SetRelativeRotation` (`self.SpringArm`) (`KismetMathLibrary.MakeRotator` 0.0 (.y _output_get)) false false))

(event `self.ReceiveBeginPlay`
  ; 2단 점프
  (set `self.SecondJumpVelocity` (`KismetMathLibrary.FTrunc` (`CharacterMovementComponent.JumpZVelocity` (`self.CharacterMovement`))))
  ; 회전 초기화
  (bind _output_get (set `self.CurrentCameraRelativeRot` (0.0 0.0 0.0)))
  (`SceneComponent.K2_SetRelativeRotation` (`self.SpringArm`) (`KismetMathLibrary.Conv_VectorToRotator` _output_get) false false)
  (`SceneComponent.K2_SetRelativeRotation` (`self.Aim`) (`KismetMathLibrary.Conv_VectorToRotator` _output_get) false false))

(event `Key|SpaceBar`
  (params (Key :type "Key Structure"))
  ; 2단 점프
  (:`Pressed`
    (if (`self.CanJump`)
      (set `self.JumpTimes` 2))
    (switch `int` (`self.JumpTimes`)
      (:`1`
        (set `self.JumpTimes` (- (`self.JumpTimes`) 1))
        (`self.LaunchCharacter` (`KismetMathLibrary.MakeVector` 0.0 0.0 (`KismetMathLibrary.Conv_IntToDouble` (`self.SecondJumpVelocity`)))))
      (:`2`
        (set `self.JumpTimes` (- (`self.JumpTimes`) 1))
        (`self.Jump`)))))

(event `self.ReceiveTick`
  (params (DeltaSeconds :type "Float (single-precision)"))
  (bind _aim (`self.Aim`))
  (bind _direction (`self.Direction`))
  (set `self.Direction` (* (`KismetMathLibrary.Normal` (+ (* (`SceneComponent.GetForwardVector` _aim) (`self.GetInputAxisValue`)) (* (`SceneComponent.GetRightVector` _aim) (`self.GetInputAxisValue`)))) (`self.Speed`) (`GameplayStatics.GetWorldDeltaSeconds`)))
  (if (> (`KismetMathLibrary.VSize` _direction) 0.0)
    (`self.K2_SetActorLocation` (+ (`self.K2_GetActorLocation`) _direction) true)
    (`SceneComponent.K2_SetRelativeRotation` (`self.Mesh`) (`KismetMathLibrary.MakeRotFromXZ` (`SceneComponent.GetForwardVector` (`self.Aim`)) (`self.GetActorUpVector`)) false false)))

(fn `UserConstructionScript`)