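; ProjectSD game mode that tallies combat stats and shows the end-of-game result screen.
; Events accumulate damage dealt, damage taken, rifle kills and skill kills.
; GameClear flags the game as set and fades in WBP_GameOverUI with the boss's play time and totals, though three totals land in differently named text fields.
; OpenLoading shows a loading widget, then opens LjgTestMap after a short delay.
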(event `self.ReceiveBeginPlay`)

(event `OpenLoading`
  ; 게임결과창 로직
  (bind _returnvalue (`|CreateWidget` "/Game/ProjectSD/Blueprints/UI/Loading/WBP_LoadingUI.WBP_LoadingUI_C" (`GameplayStatics.GetPlayerController` 0)))
  (`UserWidget.AddToViewport` _returnvalue 0)
  (`KismetSystemLibrary.Delay` 3.0)
  (`GameplayStatics.OpenLevelBySoftObjectPtr` "/Game/ProjectSD/Maps/LJG/LjgTestMap.LjgTestMap"))

(event `GameClear`
  (params (Boss :type "/Game/ProjectSD/Blueprints/Character/Enemy/Boss/BP_GraveWalker Object Reference"))
  (bind _playtime (`/Game/ProjectSD/Blueprints/Character/Enemy/Boss/BP_GraveWalker.PlayTime` Boss))
  ; 게임결과창 로직
  (set `self.bIsGameSet` true)
  (bind _returnvalue (`|CreateWidget` "/Game/ProjectSD/Blueprints/UI/GameEnd/WBP_GameOverUI.WBP_GameOverUI_C" (`GameplayStatics.GetPlayerController` 0)))
  (`UserWidget.AddToViewport` _returnvalue 0)
  (`UserWidget.PlayAnimation` _returnvalue (`/Game/ProjectSD/Blueprints/UI/GameEnd/WBP_GameOverUI.FadeOverlay` _returnvalue) 0.0 1 "Forward" 1.0 false)
  (set `TextBlock.Text` (`KismetTextLibrary.Conv_StringToText` (`KismetStringLibrary.Concat_StrStr` (`KismetStringLibrary.Conv_Int64ToString` (`KismetMathLibrary.Conv_DoubleToInt64` (/ _playtime 60.0))) "분 " (`KismetStringLibrary.Conv_Int64ToString` (`KismetMathLibrary.Conv_DoubleToInt64` (mod _playtime 60.0))) "초")) (`/Game/ProjectSD/Blueprints/UI/GameEnd/WBP_GameOverUI.TimeText` _returnvalue))
  (set `TextBlock.Text` (`KismetTextLibrary.Conv_DoubleToText` (`self.ResultDamages`) "HalfToEven") (`/Game/ProjectSD/Blueprints/UI/GameEnd/WBP_GameOverUI.ResultDamage` _returnvalue))
  (set `TextBlock.Text` (`KismetTextLibrary.Conv_DoubleToText` (`self.ResultTakeDamages`) "HalfToEven") (`/Game/ProjectSD/Blueprints/UI/GameEnd/WBP_GameOverUI.ResultKillOfRifle` _returnvalue))
  (set `TextBlock.Text` (`KismetTextLibrary.Conv_IntToText` (`self.ResultKillsOfRifle`)) (`/Game/ProjectSD/Blueprints/UI/GameEnd/WBP_GameOverUI.ResultKillOfSkill` _returnvalue))
  (set `TextBlock.Text` (`KismetTextLibrary.Conv_IntToText` (`self.ResultKillsOfSkill`)) (`/Game/ProjectSD/Blueprints/UI/GameEnd/WBP_GameOverUI.ResultTakeDamage` _returnvalue)))

(event `ResultDamage`
  (params (Damage :type "Float (double-precision)"))
  ; 결과창 데이터 누적 이벤트
  (set `self.ResultDamages` (+ (`self.ResultDamages`) Damage)))

(event `ResultTakeDamage`
  (params (Damage :type "Float (double-precision)"))
  ; 결과창 데이터 누적 이벤트
  (set `self.ResultTakeDamages` (+ (`self.ResultTakeDamages`) Damage)))

(event `ResultKillOfRifle`
  ; 결과창 데이터 누적 이벤트
  (set `self.ResultKillsOfRifle` (+ (`self.ResultKillsOfRifle`) 1)))

(event `ResultKillOfSkill`
  ; 결과창 데이터 누적 이벤트
  (set `self.ResultKillsOfSkill` (+ (`self.ResultKillsOfSkill`) 1)))

(fn `UserConstructionScript`)